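; Lightghost is an actor whose trigger volume acts as a safe zone, with game over for staying outside too long.
; Leaving the trigger plays a timeline that drives danger camera shake through its Intensity track, and re-entering reverses it.
; When the Death track reaches one, it fades out, locks input via cinematic mode and opens GameOverScreen after a delay.
; Overlaps are not filtered by actor.
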(event `self.LightghostTrigger.OnComponentEndOverlap`
  (params (OtherActor :type "Actor Object Reference") (OtherComp :type "PrimitiveComponent Object Reference") (OtherBodyIndex :type Integer))
  (bind _playercameramanager (`PlayerController.PlayerCameraManager` (`GameplayStatics.GetPlayerController` 0)))
  (set `self.Player in bounds?` false)
  (`KismetSystemLibrary.PrintString` "OUT OF BOUNDS")
  (if (not (`self.Player in bounds?`))
    (bind (_direction _intensity _death) (`Timeline|Timeline_0` :!label _label)
      (:`Update`
        (`|ExecutionSequence`
          (:`then_0`
            (if (>= _death 1.0)
              (`PlayerCameraManager.PlayCameraShake` :`self` _playercameramanager :`ShakeClass` "/Game/CastleQuest/Blueprints/Base/DangerShake.DangerShake_C" :`Scale` 0.0)
              (`PlayerCameraManager.StartCameraFade` :`self` _playercameramanager :`ToAlpha` 1.0 :`Duration` 2.0 :`bShouldFadeAudio` true :`bHoldWhenFinished` true)
              (`PlayerController.SetCinematicMode` (`GameplayStatics.GetPlayerController` 0) true false true true true)
              (`KismetSystemLibrary.Delay` 3.0)
              (`GameplayStatics.OpenLevel` "GameOverScreen")))
          (:`then_1`
            (`PlayerCameraManager.PlayCameraShake` :`self` _playercameramanager :`ShakeClass` "/Game/CastleQuest/Blueprints/Base/DangerShake.DangerShake_C" :`Scale` _intensity)))))))

(event `self.LightghostTrigger.OnComponentBeginOverlap`
  (params (OtherActor :type "Actor Object Reference") (OtherComp :type "PrimitiveComponent Object Reference") (OtherBodyIndex :type Integer) (bFromSweep :type Boolean) (SweepResult :type "HitResult Structure (by ref)"))
  (set `self.Player in bounds?` true)
  (`KismetSystemLibrary.PrintString` "!!!!!!!!!! SAFE !!!!!!!!!!!")
  (if (`self.Player in bounds?`)
    (goto _label :!via `Reverse`)))

(fn `UserConstructionScript`)