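; Wardrobe double-door puzzle actor that stays inactive until its handles are collected, then opens to make a referenced key collectable.
; BeginPlay disables the door trigger and the key's sphere collision, and HandlesCollected re-enables the trigger.
; Tick polls the player's use button through a trigger-controlled gate into a DoOnce, which shows both handles.
; After a delay, a timeline swings the doors in opposite directions, then enables the key's collision.
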(event `self.ReceiveBeginPlay`
  (`PrimitiveComponent.SetCollisionEnabled` (`self.Door Trigger`) "NoCollision")
  (bind _asbp_locked_door_key (cast `/Game/CastleQuest/Blueprints/BP_Locked_Door_Key` (`self.Keys Reference`)))
  (`PrimitiveComponent.SetCollisionEnabled` (`/Game/CastleQuest/Blueprints/BP_Locked_Door_Key.Sphere` _asbp_locked_door_key) "NoCollision"))

(event `Handles Collected`
  (`PrimitiveComponent.SetCollisionEnabled` (`self.Door Trigger`) "QueryAndPhysics"))

(event `self.ReceiveTick`
  (params (DeltaSeconds :type "Float (single-precision)"))
  (bind _asfirst_person_character (cast `/Game/FirstPersonBP/Blueprints/FirstPersonCharacter` (`GameplayStatics.GetPlayerPawn` 0)))
  (if (`/Game/FirstPersonBP/Blueprints/FirstPersonCharacter.Use Button Pressed` _asfirst_person_character)
    (`/Engine/EditorBlueprintResources/StandardMacros.Gate` true :!label _label
      (:`Exit`
        (`/Engine/EditorBlueprintResources/StandardMacros.DoOnce` false
          (:`Completed`
            (`SceneComponent.SetVisibility` (`self.Doorhandle_R`) true false)
            (`SceneComponent.SetVisibility` (`self.DoorHandle_L`) true false)
            (`KismetSystemLibrary.Delay` 1.0)
            (bind (_direction _rotation) (`Timeline|Door Opening` :!via `PlayFromStart`)
              (:`Update`
                (`SceneComponent.K2_SetRelativeRotation` (`self.door_R`) (`KismetMathLibrary.MakeRotator` 0.0 0.0 _rotation) false false)
                (`SceneComponent.K2_SetRelativeRotation` (`self.door_L`) (`KismetMathLibrary.MakeRotator` 0.0 0.0 (* _rotation -1.0)) false false))
              (:`Finished`
                (bind _asbp_locked_door_key (cast `/Game/CastleQuest/Blueprints/BP_Locked_Door_Key` (`self.Keys Reference`)))
                (`PrimitiveComponent.SetCollisionEnabled` (`/Game/CastleQuest/Blueprints/BP_Locked_Door_Key.Sphere` _asbp_locked_door_key) "QueryAndPhysics")))))))))

(event `self.Door Trigger.OnComponentBeginOverlap`
  (params (OtherActor :type "Actor Object Reference") (OtherComp :type "PrimitiveComponent Object Reference") (OtherBodyIndex :type Integer) (bFromSweep :type Boolean) (SweepResult :type "HitResult Structure (by ref)"))
  (goto _label :!via `Open`))

(event `self.Door Trigger.OnComponentEndOverlap`
  (params (OtherActor :type "Actor Object Reference") (OtherComp :type "PrimitiveComponent Object Reference") (OtherBodyIndex :type Integer))
  (goto _label :!via `Close`))

(fn `UserConstructionScript`)