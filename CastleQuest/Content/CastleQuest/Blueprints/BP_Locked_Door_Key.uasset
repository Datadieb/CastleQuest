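; Key pickup that unlocks its assigned target door when the player presses use nearby.
; Sphere overlaps open and close a gate, without filtering the overlapping actor, while Tick polls the first-person character's use-button flag.
; When the press passes the gate, the key marks itself collected, flags the door as unlocked and destroys itself after a short delay.
; The construction script applies the configurable mesh.
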(event `self.ReceiveTick`
  (params (DeltaSeconds :type "Float (single-precision)"))
  (bind _asfirst_person_character (cast `/Game/FirstPersonBP/Blueprints/FirstPersonCharacter` (`GameplayStatics.GetPlayerPawn` 0) :!label _label))
  (if (`/Game/FirstPersonBP/Blueprints/FirstPersonCharacter.Use Button Pressed` _asfirst_person_character)
    (`/Engine/EditorBlueprintResources/StandardMacros.Gate` true :!label _label_2
      (:`Exit`
        (set `self.Is Collected?` true)
        (set `/Game/CastleQuest/Blueprints/BP_Locked_Door.Unlocked Door with Key?` true (`self.Target Door`))
        (`KismetSystemLibrary.Delay` 0.05)
        (`self.K2_DestroyActor`)))))

(event `self.Sphere.OnComponentBeginOverlap`
  (params (OtherActor :type "Actor Object Reference") (OtherComp :type "PrimitiveComponent Object Reference") (OtherBodyIndex :type Integer) (bFromSweep :type Boolean) (SweepResult :type "HitResult Structure (by ref)"))
  (`|ExecutionSequence`
    (:`then_0`
      (goto _label))
    (:`then_1`
      (goto _label_2 :!via `Open`))))

(event `self.Sphere.OnComponentEndOverlap`
  (params (OtherActor :type "Actor Object Reference") (OtherComp :type "PrimitiveComponent Object Reference") (OtherBodyIndex :type Integer))
  (goto _label_2 :!via `Close`))

(fn `UserConstructionScript`
  (`StaticMeshComponent.SetStaticMesh` (`self.KeyMesh`) (`self.Mesh`)))