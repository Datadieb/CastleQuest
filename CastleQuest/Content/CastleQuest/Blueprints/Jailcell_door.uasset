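; Jail cell door Blueprint that plays a squeak sound when the door component is hit.
; A DoOnce gates the hit response, which fades the squeak audio in, holds briefly, then fades it out, while a parallel delayed branch resets the gate to limit retriggering.
; A scare trigger event calls AddForceAtLocation on the door, though its force and location are both zero vectors.
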(event `self.jailcell_door01.OnComponentHit`
  (params (OtherActor :type "Actor Object Reference") (OtherComp :type "PrimitiveComponent Object Reference") (NormalImpulse :type "Vector Structure") (Hit :type "HitResult Structure (by ref)"))
  (bind _doorsqueak (`self.doorsqueak`))
  (`|ExecutionSequence`
    (:`then_0`
      (`/Engine/EditorBlueprintResources/StandardMacros.DoOnce` false :!label _label
        (:`Completed`
          (`AudioComponent.SetVolumeMultiplier` _doorsqueak (* 1.0 1.0))
          (`ActorComponent.SetActive` _doorsqueak false false)
          (`AudioComponent.FadeIn` _doorsqueak 0.5 1.0 0.0)
          (`KismetSystemLibrary.Delay` 1.0)
          (`AudioComponent.FadeOut` _doorsqueak 0.5 0.0))))
    (:`then_1`
      (`KismetSystemLibrary.Delay` 1.8)
      (goto _label :!via `Reset`))))

(event `ScareTrigger_triggered_Event`
  (`PrimitiveComponent.AddForceAtLocation` (`self.jailcell_door01`) (0.0 0.0 0.0) (0.0 0.0 0.0) "None"))

(fn `UserConstructionScript`)