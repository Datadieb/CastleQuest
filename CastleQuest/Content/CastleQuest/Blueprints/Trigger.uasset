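; Interactive lantern trigger that sets its PointLight's visibility when the player presses use within range.
; Overlap begin and end on TriggerPrimitive open and close a Gate, without filtering which actor overlaps.
; Tick polls the FirstPersonCharacter's UseButtonPressed flag through that Gate, applying the Visibility variable to the light and calling NewLanternLitEvent on the character.
; The Gate stays open after firing, so this repeats every frame the flag remains true.
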(event `self.ReceiveTick`
  (params (DeltaSeconds :type "Float (single-precision)"))
  ;[1 1 1] Check if player pressed the use button
  (bind _asfirst_person_character (cast `/Game/FirstPersonBP/Blueprints/FirstPersonCharacter` (`GameplayStatics.GetPlayerPawn` 0)))
  (if (`/Game/FirstPersonBP/Blueprints/FirstPersonCharacter.Use Button Pressed` _asfirst_person_character)
    ;[1 1 1] Check if player is within range and toggle visibility on PC lantern.
    (`/Engine/EditorBlueprintResources/StandardMacros.Gate` true :!label _label
      (:`Exit`
        (`SceneComponent.SetVisibility` (`self.PointLight`) (`self.Visibility`) false)
        (bind _asfirst_person_character_2 (cast `/Game/FirstPersonBP/Blueprints/FirstPersonCharacter` (`GameplayStatics.GetPlayerPawn` 0)))
        (`/Game/FirstPersonBP/Blueprints/FirstPersonCharacter.New Lantern Lit?_Event` _asfirst_person_character_2)))))

(event `self.TriggerPrimitive.OnComponentBeginOverlap`
  (params (OtherActor :type "Actor Object Reference") (OtherComp :type "PrimitiveComponent Object Reference") (OtherBodyIndex :type Integer) (bFromSweep :type Boolean) (SweepResult :type "HitResult Structure (by ref)"))
  ;[1 1 1] Generate Overlap range checks
  (goto _label :!via `Open`))

(event `self.TriggerPrimitive.OnComponentEndOverlap`
  (params (OtherActor :type "Actor Object Reference") (OtherComp :type "PrimitiveComponent Object Reference") (OtherBodyIndex :type Integer))
  ;[1 1 1] Generate Overlap range checks
  (goto _label :!via `Close`))

(fn `UserConstructionScript`)