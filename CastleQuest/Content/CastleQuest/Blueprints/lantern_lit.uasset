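; Lantern Blueprint for CastleQuest with a point light that can be lit or unlit and can flicker.
; The construction script sets the light to its Intensity when Lit, or hides it otherwise.
; On BeginPlay, if flickering is enabled, a timeline track scales Intensity to animate the light's brightness; otherwise the timeline is stopped.
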(event `self.ReceiveBeginPlay`
  (if (`self.Flickering?`)
    (bind (_direction _newtrack_0) (`Timeline|Flickering` :!label _label)
      (:`Update`
        (`LightComponent.SetIntensity` (`self.PointLight`) (* _newtrack_0 (`self.Intensity`)))))
    (else
      (goto _label :!via `Stop`))))

(fn `UserConstructionScript`
  (bind _pointlight (`self.PointLight`))
  (if (`self.Lit?`)
    (`LightComponent.SetIntensity` _pointlight (`self.Intensity`))
    (else
      (`SceneComponent.SetVisibility` _pointlight false false))))