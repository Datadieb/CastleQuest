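; Scare01_JailDoors is a one-shot scare trigger that, going by its name and audio, shoves jail doors with a squeak.
; A gate on the box overlap opens only when the lantern event reports the player has it.
; The first overlap through the gate sets RadialForce strengths, fires an impulse and fades in the squeak sound.
; After a ten-second delay it fades the sound out and destroys itself.
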(event `self.Box.OnComponentBeginOverlap`
  (params (OtherActor :type "Actor Object Reference") (OtherComp :type "PrimitiveComponent Object Reference") (OtherBodyIndex :type Integer) (bFromSweep :type Boolean) (SweepResult :type "HitResult Structure (by ref)"))
  (bind _sfx_scaredoorsqueak (`self.SFX_ScareDoorSqueak`))
  (bind _radialforce (`self.RadialForce`))
  (`/Engine/EditorBlueprintResources/StandardMacros.Gate` true :!label _label
    (:`Exit`
      (`KismetSystemLibrary.PrintString` "Force")
      (`/Engine/EditorBlueprintResources/StandardMacros.DoOnce` false
        (:`Completed`
          (`|ExecutionSequence`
            (:`then_0`
              (set `RadialForceComponent.ImpulseStrength` (`self.Impulse`) _radialforce))
            (:`then_1`
              (set `RadialForceComponent.ForceStrength` (`self.Strength`) _radialforce))
            (:`then_2`
              (`|ExecutionSequence`
                (:`then_0`
                  (`/Engine/EditorBlueprintResources/StandardMacros.DoOnce` false :!label _label_2
                    (:`Completed`
                      (`AudioComponent.SetVolumeMultiplier` _sfx_scaredoorsqueak (* 1.0 1.0))
                      (`RadialForceComponent.FireImpulse` (`self.RadialForce`))
                      (`ActorComponent.SetActive` _sfx_scaredoorsqueak true false)
                      (`AudioComponent.FadeIn` _sfx_scaredoorsqueak 0.5 1.0 0.0)
                      (`KismetSystemLibrary.Delay` 10.0)
                      (`AudioComponent.FadeOut` _sfx_scaredoorsqueak 0.5 0.0)
                      (`self.K2_DestroyActor`))))
                (:`then_1`
                  (`KismetSystemLibrary.Delay` 1.8)
                  (goto _label_2 :!via `Reset`))))))))))

(event `PlayerhasLantern?_Event`
  (params (`Active?` :type Boolean))
  (if `Active?`
    (goto _label :!via `Open`)))

(fn `UserConstructionScript`)