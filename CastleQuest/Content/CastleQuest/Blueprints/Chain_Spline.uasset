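; Spline-driven chain builder that lays deformed chain meshes along an editable spline at construction time, with an optional closed loop.
; The construction script resizes a per-point data array to match the spline points, then adds a spline mesh component for each segment.
; Per-point data sets roll, width and thickness at segment ends and toggles up to four additional meshes, with optional collision on every piece.
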(event EventBeginPlay)

(event EventActorBeginOverlap
  (params (OtherActor :type Actor%20Object%20Reference)))

(event EventTick
  (params (DeltaSeconds :type Float%20%28single-precision%29)))

(fn ConstructionScript
  (Utilities|FlowControl|Sequence
    (:then_0
      (|StoreNumbertoSplinePoints))
    (:then_1
      (|BuildDataArray))
    (:then_2
      (|ConstructionLoop)
      (|StoreDrawAdditionalMeshes)
      (Utilities|FlowControl|Sequence
        (:then_0
          (CallFunction|BuildTrackElements (Variables|Default|GetCurrentLoopIndex) (Variables|Default|GetChainMesh)))
        (:then_1
          (if (Variables|Default|GetDrawFirstAdditionalMesh)
            (CallFunction|BuildTrackElements (Variables|Default|GetCurrentLoopIndex) (Variables|Default|GetFirstAdditionalMesh))))
        (:then_2
          (if (Variables|Default|GetDrawSecondAdditionalMesh)
            (CallFunction|BuildTrackElements (Variables|Default|GetCurrentLoopIndex) (Variables|Default|GetSecondAdditionalMesh))))
        (:then_3
          (if (Variables|Default|GetDrawThirdAdditionalMesh)
            (CallFunction|BuildTrackElements (Variables|Default|GetCurrentLoopIndex) (Variables|Default|GetThirdAdditionalMesh))))
        (:then_4
          (if (Variables|Default|GetDrawFourthAdditonalMesh)
            (CallFunction|BuildTrackElements (Variables|Default|GetCurrentLoopIndex) (Variables|Default|GetFourthAdditionalMesh))))))))

(fn BuildTrackElements
  (params (Loop%20Index :type Integer) (Track%20Element%20Mesh :type Static%20Mesh%20Object%20Reference))
  (LocalVariables|SetLocal%20Current%20Loop%20Index Loop%20Index)
  (LocalVariables|SetLocal%20Next%20Loop%20Index (Math|Integer|%(Integer) (+ Loop%20Index 1) (Variables|Default|GetSpline%20Point%20Numbers)))
  (LocalVariables|SetLocal%20Track%20Element%20Mesh Track%20Element%20Mesh)
  (Utilities|FlowControl|Sequence
    (:then_0
      (LocalVariables|SetLocal%20Start%20Location (.Location (Spline|GetLocationandTangentatSplinePoint (Variables|Default|GetSpline) (LocalVariables|GetLocal%20Current%20Loop%20Index) "Local")))
      (LocalVariables|SetLocal%20Start%20Tangent (.Tangent (Spline|GetLocationandTangentatSplinePoint (Variables|Default|GetSpline) (LocalVariables|GetLocal%20Current%20Loop%20Index) "Local")))
      (LocalVariables|SetLocal%20End%20Location (.Location (Spline|GetLocationandTangentatSplinePoint (Variables|Default|GetSpline) (LocalVariables|GetLocal%20Next%20Loop%20Index) "Local")))
      (LocalVariables|SetLocal%20End%20Tangent (.Tangent (Spline|GetLocationandTangentatSplinePoint (Variables|Default|GetSpline) (LocalVariables|GetLocal%20Next%20Loop%20Index) "Local")))
      (LocalVariables|SetLocal%20Start%20Roll (.chainroll (Utilities|Array|Get(acopy) (Variables|Default|GetRoadDataArray) (LocalVariables|GetLocal%20Current%20Loop%20Index))))
      (LocalVariables|SetLocal%20Start%20Scale (Math|Vector2D|MakeVector2D (.chainwidth (Utilities|Array|Get(acopy) (Variables|Default|GetRoadDataArray) (LocalVariables|GetLocal%20Current%20Loop%20Index))) (.chainthickness (Utilities|Array|Get(acopy) (Variables|Default|GetRoadDataArray) (LocalVariables|GetLocal%20Current%20Loop%20Index)))))
      (LocalVariables|SetLocal%20End%20Roll (.chainroll (Utilities|Array|Get(acopy) (Variables|Default|GetRoadDataArray) (LocalVariables|GetLocal%20Next%20Loop%20Index))))
      (LocalVariables|SetLocal%20End%20Scale (Math|Vector2D|MakeVector2D (.chainwidth (Utilities|Array|Get(acopy) (Variables|Default|GetRoadDataArray) (LocalVariables|GetLocal%20Next%20Loop%20Index))) (.chainthickness (Utilities|Array|Get(acopy) (Variables|Default|GetRoadDataArray) (LocalVariables|GetLocal%20Next%20Loop%20Index))))))
    (:then_1
      (bind _returnvalue (AddComponent|AddSplineMeshComponent false))
      (bind _output_get (LocalVariables|SetLocal%20Current%20Spline%20Mesh _returnvalue))
      (Components|StaticMesh|SetStaticMesh _output_get (LocalVariables|GetLocal%20Track%20Element%20Mesh))
      (SplineMesh|SetStartandEnd (LocalVariables|GetLocal%20Current%20Spline%20Mesh) (LocalVariables|GetLocal%20Start%20Location) (LocalVariables|GetLocal%20Start%20Tangent) (LocalVariables|GetLocal%20End%20Location) (LocalVariables|GetLocal%20End%20Tangent) true :!class /Script/Engine.SplineMeshComponent)
      (Class|SplineMeshComponent|SetStartRoll (LocalVariables|GetLocal%20Current%20Spline%20Mesh) (LocalVariables|GetLocal%20Start%20Roll) true)
      (Class|SplineMeshComponent|SetEndRoll (LocalVariables|GetLocal%20Current%20Spline%20Mesh) (LocalVariables|GetLocal%20End%20Roll) true)
      (SplineMesh|SetStartScale (LocalVariables|GetLocal%20Current%20Spline%20Mesh) (LocalVariables|GetLocal%20Start%20Scale) true :!class /Script/Engine.SplineMeshComponent)
      (SplineMesh|SetEndScale (LocalVariables|GetLocal%20Current%20Spline%20Mesh) (LocalVariables|GetLocal%20End%20Scale) true :!class /Script/Engine.SplineMeshComponent)
      (Collision|SetCollisionEnabled (LocalVariables|GetLocal%20Current%20Spline%20Mesh) (select (Variables|Default|GetCollision) "QueryAndPhysics" "NoCollision")))))